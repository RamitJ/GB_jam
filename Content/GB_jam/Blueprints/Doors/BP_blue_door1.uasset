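; Blue door Blueprint that swings open when a first-person character holding the blue key overlaps its trigger box.
; A Door_rotation timeline lerps the mesh's yaw between closed and opened values, then toggles IsOpened when finished.
; Without the key, it shows a door-locked widget, then removes all widgets of that class after a short delay.
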(event OnComponentBeginOverlap(Box1)
  (params (OverlappedComponent :type Primitive%20Component%20Object%20Reference) (OtherActor :type Actor%20Object%20Reference) (OtherComp :type Primitive%20Component%20Object%20Reference) (OtherBodyIndex :type Integer) (bFromSweep :type Boolean) (SweepResult :type Hit%20Result%20Structure%20%28by%20ref%29))
  (bind _asbp_first_person_character (Utilities|Casting|CastToBP_FirstPersonCharacter OtherActor))
  (if (Variables|/Game/FirstPerson/Blueprints/BP_FirstPersonCharacter.BP_FirstPersonCharacter_C|GetHasBlueKey _asbp_first_person_character)
    (bind _door_track (Timeline|Door_rotation Play)
      (:Update
        (Transformation|SetRelativeRotation (Variables|Default|GetStaticMesh) (Math|Rotator|MakeRotator 0.0 0.0 (Math|Float|Lerp (Variables|Default|GetDoorClosed) (Variables|Default|GetDoorOpened) _door_track)) false false))
      (:Finished
        (Variables|Default|SetIsOpened? (not (Variables|Default|GetIsOpened?)))))
    (else
      (bind _returnvalue (UserInterface|CreateWidget "/Game/GB_jam/Widgets/BPI_door_locked.BPI_door_locked_C"))
      (UserInterface|Viewport|AddtoViewport _returnvalue 0)
      (Utilities|FlowControl|Delay 3.0)
      (Utilities|Casting|CastToPawn (Game|Player|GetPlayerPawn 0))
      (bind _foundwidgets (Widget|GetAllWidgetsOfClass "/Game/GB_jam/Widgets/BPI_door_locked.BPI_door_locked_C" true))
      (Widget|RemovefromParent _foundwidgets))))

(event EventBeginPlay)

(event Collision|EventActorBeginOverlap
  (params (OtherActor :type Actor%20Object%20Reference)))

(event EventTick
  (params (DeltaSeconds :type Float%20%28single-precision%29)))

(fn ConstructionScript)